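; Jammer actor that endlessly flies a fixed rectangular patrol loop around its spawn point; the file holds no jamming logic.
; BeginPlay stores the start location and calls startCursing, which chains timed MoveComponentTo moves on the root, alternating straight legs with quick quarter turns at the corners.
; The path ends back at the start location, then repeats after a short delay without using Tick.
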(event Custom|startCursing
  (bind _startlocation (Variables|Default|GetstartLocation))
  (bind _root (Variables|Default|GetRoot))
  (bind _returnvalue (+ _startlocation "20000.000000, 0, 0"))
  (bind _returnvalue_2 (+ _startlocation "20000.000000,-10000.000000, 0"))
  (bind _returnvalue_3 (+ _startlocation "-20000.000000,-10000.000000, 0"))
  (bind _returnvalue_4 (+ _startlocation "-20000.000000,0.000000, 0"))
  (Components|MoveComponentTo _root _returnvalue "0,0.000000, 0" false false 1e+01 false :!label _label)
  (Components|MoveComponentTo _root _returnvalue "0,270.000000, 0" false false 0.5 false)
  (Components|MoveComponentTo _root _returnvalue_2 "0,270.000000, 0" false false 5.0 false)
  (Components|MoveComponentTo _root _returnvalue_2 "0,180.000000, 0" false false 0.5 false)
  (Components|MoveComponentTo _root _returnvalue_3 "0,180.000000, 0" false false 1e+01 false)
  (Components|MoveComponentTo _root _returnvalue_3 "0,90.000000, 0" false false 0.5 false)
  (Components|MoveComponentTo _root _returnvalue_4 "0,90.000000, 0" false false 5.0 false)
  (Components|MoveComponentTo _root _returnvalue_4 "0,0.000000, 0" false false 0.5 false)
  (Components|MoveComponentTo _root (+ _startlocation "0.000000,0.000000, 0") "0, 0, 0" false false 1e+01 false)
  (Utilities|FlowControl|Delay 0.1)
  (goto _label))

(event EventBeginPlay
  (Variables|Default|SetstartLocation (Transformation|GetActorLocation))
  (CallFunction|StartCursing))

(event Collision|EventActorBeginOverlap
  (params (OtherActor :type Actor%20Object%20Reference)))

(event EventTick
  (params (DeltaSeconds :type Float%20%28single-precision%29)))

(fn ConstructionScript)