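; Radar_Return_BP is a component for the 3D radar that resolves which scene components on its owning actor it refers to.
; On BeginPlay it targets the owner's root component, or the first scene component whose name contains the ApplyToComponent keyword when one is set.
; Only in that keyword case, it also searches by the optional ScaleFromRootComponent keyword for a relative root to scale from.
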(event EventBeginPlay
  ;[1 1 1] Locate the component on the parent actor that contains the provided keyword in its name
  (if (Utilities|Enum|Equal(Enum) (Variables|Default|GetApply%20To%20Component) "")
    (Variables|Default|SetApplies%20To%20Component (Variables|/Script/Engine.Actor|GetRootComponent (Components|GetOwner)))
    (else
      (bind _array_element (Utilities|Array|ForEachLoopwithBreak (Actor|GetComponentsByClass (Components|GetOwner) "/Script/Engine.SceneComponent") :!label _label)
        (:LoopBody
          (if (Utilities|String|Contains (Utilities|GetObjectName _array_element) (Variables|Default|GetApply%20To%20Component))
            (Variables|Default|SetApplies%20To%20Component _array_element)
            (goto _label Break)))
        (:Completed
          ;[1 1 1] Locate a relative root component to scale up from.
          (if (not (Utilities|Enum|Equal(Enum) (Variables|Default|GetScale%20From%20Root%20Component) ""))
            (bind _array_element_2 (Utilities|Array|ForEachLoopwithBreak (Actor|GetComponentsByClass (Components|GetOwner) "/Script/Engine.SceneComponent") :!label _label_2)
              (:LoopBody
                (if (Utilities|String|Contains (Utilities|GetObjectName _array_element_2) (Variables|Default|GetScale%20From%20Root%20Component))
                  (Variables|Default|SetScale%20From%20Component _array_element_2)
                  (goto _label_2 Break))))))))))