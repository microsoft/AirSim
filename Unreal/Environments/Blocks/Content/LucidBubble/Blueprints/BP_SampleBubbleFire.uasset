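; BP_SampleBubbleFire is a sample emitter actor that fires bubbles at random intervals until game time passes GenEventTime, then disables its tick.
; Tick counts down NextGenTime, then rerolls it through ResetTime and calls CreateBubble.
; CreateBubble spawns a BubbleClass actor at the root with random uniform scale, a random material from BubbleMaterials and a direction within an elliptical cone around forward.
; Each valid bubble is launched through Fire at a random velocity.
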(event EventBeginPlay)

(event Collision|EventActorBeginOverlap
  (params (OtherActor :type Actor%20Object%20Reference)))

(event EventTick
  (params (DeltaSeconds :type Float%20%28single-precision%29))
  (|CallParentFunction DeltaSeconds)
  (if (<= (Utilities|Time|GetGameTimeinSeconds) (Variables|Default|GetGenEventTime))
    (Utilities|FlowControl|Sequence
      (:then_0
        (Variables|Default|SetNextGenTime (- (Variables|Default|GetNextGenTime) DeltaSeconds)))
      (:then_1
        (if (<= (Variables|Default|GetNextGenTime) 0.0)
          (CallFunction|ResetTime)
          (bind _returnvalue (CallFunction|CreateBubble))
          (Utilities|IsValid _returnvalue
            (:Is%20Valid
              (Default|Fire _returnvalue (Math|Random|RandomFloatinRange (Variables|Default|GetFireVelocityMin) (Variables|Default|GetFireVelocityMax))))))))
    (else
      (Actor|Tick|SetActorTickEnabled false))))

(fn ConstructionScript)

(fn ResetTime
  (Variables|Default|SetNextGenTime (Math|Random|RandomFloatinRange (Variables|Default|GetGentimeMin) (Variables|Default|GetGentimeMax))))

(fn CreateBubble
  (bind _defaultsceneroot (Variables|Default|GetDefaultSceneRoot))
  (bind _returnvalue (Transformation|GetWorldRotation _defaultsceneroot))
  (LocalVariables|SetScale (Math|Random|RandomFloatinRange (Variables|Default|GetBubbleSizeMin) (Variables|Default|GetBubbleSizeMax)))
  (bind _returnvalue_2 (Game|SpawnActorfromClass (Variables|Default|GetBubbleClass) (Math|Transform|MakeTransform (Transformation|GetWorldLocation (Variables|Default|GetDefaultSceneRoot)) (Math|Rotator|MakeRotfromXZ (Class|KismetMathLibrary|RandomUnitVectorinEllipticalConeinDegrees (Math|Vector|GetForwardVector _returnvalue) (Variables|Default|GetFireRangeYaw) (Variables|Default|GetFireRangePitch)) (Math|Vector|GetUpVector _returnvalue)) (Math|Vector|MakeVector (LocalVariables|GetScale) (LocalVariables|GetScale) (LocalVariables|GetScale))) "AlwaysSpawn" 0 (CallFunction|GetMaterial) 0))
  (return _returnvalue_2))

(fn GetMaterial
  (if (> (Utilities|Array|Length (Variables|Default|GetBubbleMaterials)) 0)
    (return (Utilities|Array|Get(acopy) (Variables|Default|GetBubbleMaterials) (Math|Random|RandomIntegerinRange 0 (Utilities|Array|LastIndex (Variables|Default|GetBubbleMaterials)))))
    (else
      (return 0))))